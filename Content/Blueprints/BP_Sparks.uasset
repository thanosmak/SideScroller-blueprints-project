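; BP_Sparks is a side-scroller hazard that damages and briefly shocks any SideScrollerCharacter entering its box.
; On overlap it applies damage, then polls with a short delay loop until the character stops falling.
; It then forces a hurt hop by temporarily swapping jump velocity.
; After restoring jump height, it sets a random reduced walk speed for ShockDuration, then resets it to a hardcoded default.
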(event OnComponentBeginOverlap(Box)
  (params (OverlappedComponent :type Primitive%20Component%20Object%20Reference) (OtherActor :type Actor%20Object%20Reference) (OtherComp :type Primitive%20Component%20Object%20Reference) (OtherBodyIndex :type Integer) (bFromSweep :type Boolean) (SweepResult :type Hit%20Result%20Structure%20%28by%20ref%29))
  (bind _asside_scroller_character (Utilities|Casting|CastToSideScrollerCharacter OtherActor))
  (Game|Damage|ApplyDamage _asside_scroller_character 5.0 0 0)
  (if (AI|Components|NavMovement|IsFalling (Variables|/Script/Engine.Character|GetCharacterMovement _asside_scroller_character)) :!label _label
    (Utilities|FlowControl|Delay 0.1)
    (goto _label)
    (else
      (Variables|/Script/Engine.CharacterMovementComponent|SetJumpZVelocity (Variables|/Script/Engine.Character|GetCharacterMovement _asside_scroller_character) (Variables|/Game/SideScrollerBP/Blueprints/SideScrollerCharacter.SideScrollerCharacter_C|GetHurtJumpHeight _asside_scroller_character))
      (Character|Jump _asside_scroller_character)
      (Utilities|FlowControl|Delay 0.2)
      (Variables|/Script/Engine.CharacterMovementComponent|SetJumpZVelocity (Variables|/Script/Engine.Character|GetCharacterMovement _asside_scroller_character) (Variables|/Game/SideScrollerBP/Blueprints/SideScrollerCharacter.SideScrollerCharacter_C|GetJumpHeight _asside_scroller_character))
      (Variables|/Script/Engine.CharacterMovementComponent|SetMaxWalkSpeed (Variables|/Script/Engine.Character|GetCharacterMovement _asside_scroller_character) (Math|Random|RandomFloatinRange 2e+02 4e+02))
      (Utilities|FlowControl|Delay (Variables|Default|GetShockDuration))
      (Variables|/Script/Engine.CharacterMovementComponent|SetMaxWalkSpeed (Variables|/Script/Engine.Character|GetCharacterMovement _asside_scroller_character) 6e+02))))

(event OnComponentEndOverlap(Box)
  (params (OverlappedComponent :type Primitive%20Component%20Object%20Reference) (OtherActor :type Actor%20Object%20Reference) (OtherComp :type Primitive%20Component%20Object%20Reference) (OtherBodyIndex :type Integer)))

(event EventBeginPlay)

(event Collision|EventActorBeginOverlap
  (params (OtherActor :type Actor%20Object%20Reference)))

(event EventTick
  (params (DeltaSeconds :type Float%20%28single-precision%29)))

(fn ConstructionScript)